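; Ice power-up pickup that triggers the bubble player's ice effect on touch.
; A timeline drives the circle mesh's relative height, while Tick spins it by a fixed, frame-rate-dependent step.
; Capsule overlap casts to BP_Bubble_Player, calls IceEvent and destroys the pickup.
; An unconnected BPI_Interact path with DoOnce and PowerUp never runs, and a debug print remains on overlap.
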(event `self.ReceiveBeginPlay`
  (bind (_direction _newtrack_0) (`Timeline|Timeline`)
    (:`Update`
      (`SceneComponent.K2_SetRelativeLocation` (`self.SM_ice_PowerUp_Circle`) (`KismetMathLibrary.MakeVector` 0.0 0.0 (* _newtrack_0 100.0)) false false))))

(event `self.ReceiveTick`
  (params (DeltaSeconds :type "Float (single-precision)"))
  (`SceneComponent.K2_AddLocalRotation` (`self.SM_ice_PowerUp_Circle`) (struct :`Yaw` 3.0) false false))

(event `self.Capsule.OnComponentBeginOverlap`
  (params (OverlappedComponent :type "PrimitiveComponent Object Reference") (OtherActor :type "Actor Object Reference") (OtherComp :type "PrimitiveComponent Object Reference") (OtherBodyIndex :type Integer) (bFromSweep :type Boolean) (SweepResult :type "HitResult Structure (by ref)"))
  (`KismetSystemLibrary.PrintString` "Hit Ice")
  (bind _asbp_bubble_player (cast `/Game/Blueprints/Character/BP_Bubble_Player` OtherActor))
  (`/Game/Blueprints/Character/BP_Bubble_Player.Ice_Event` _asbp_bubble_player)
  (`self.K2_DestroyActor`))

(fn `UserConstructionScript`)