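; Enemy actor that, once hit, turns into an energy pickup that restores the life of the Bubble actor.
; Any HitBox overlap subtracts life but always hides the body, disables the hitbox and enables the pickup, even if life remains.
; Bubble overlapping the pickup calls LifeRestore and destroys the enemy.
; Aim-and-fire logic for spawning EnemyProjectile1 at Bubble exists but is disconnected, and Tick is empty.
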(event `self.ReceiveBeginPlay`
  (`GameplayStatics.GetAllActorsOfClass` "/Game/Blueprints/Level/Projectile.Projectile_C")
  (bind _returnvalue (`GameplayStatics.GetActorOfClass` "/Game/Blueprints/Character/Bubble.Bubble_C"))
  (set `self.BubbleREF` _returnvalue)
  (`PrimitiveComponent.SetCollisionEnabled` (`self.Energy life Collision`) "NoCollision"))

(event `self.HitBox.OnComponentBeginOverlap`
  (params (OverlappedComponent :type "PrimitiveComponent Object Reference") (OtherActor :type "Actor Object Reference") (OtherComp :type "PrimitiveComponent Object Reference") (OtherBodyIndex :type Integer) (bFromSweep :type Boolean) (SweepResult :type "HitResult Structure (by ref)"))
  (bind _hitbox (`self.HitBox`))
  ;[0 0 0] Get ht
  (`|ExecutionSequence`
    (:`then_0`
      (bind _output_get (set `self.Enemy Life` (- (`self.Enemy Life`) 20.0)))
      (if (<= _output_get 0.0)
        (set `self.Is dead?` true)
        (`SceneComponent.SetVisibility` (`self.ProjectileSpawnPoint`) false false)))
    (:`then_1`
      (`SceneComponent.SetHiddenInGame` (`self.Cube`) true false)
      (`SceneComponent.SetHiddenInGame` (`self.Cube1`) true false)
      (`SceneComponent.SetHiddenInGame` (`self.Sphere`) true false)
      (`SceneComponent.SetVisibility` (`self.Lifepickup`) false false)
      (`SceneComponent.SetVisibility` _hitbox false false)
      (`PrimitiveComponent.SetCollisionEnabled` _hitbox "NoCollision")
      (`self.Energy spawn`))))

(event `self.Energy life Collision.OnComponentBeginOverlap`
  (params (OverlappedComponent :type "PrimitiveComponent Object Reference") (OtherActor :type "Actor Object Reference") (OtherComp :type "PrimitiveComponent Object Reference") (OtherBodyIndex :type Integer) (bFromSweep :type Boolean) (SweepResult :type "HitResult Structure (by ref)"))
  ;[0 0 0] Energy restore
  (if (== OtherActor (`self.BubbleREF`))
    (`/Game/Blueprints/Character/Bubble.Life restore` (`self.BubbleREF`))
    (`self.K2_DestroyActor`)))

(event `Energy spawn`
  (`PrimitiveComponent.SetCollisionEnabled` (`self.Energy life Collision`) "QueryOnly")
  (`SceneComponent.SetVisibility` (`self.Lifepickup`) true false)
  (`SceneComponent.SetVisibility` (`self.Energy life Collision`) true false))

(event `self.ReceiveTick`
  (params (DeltaSeconds :type "Float (single-precision)"))
  ;[0 0 0] Shooting
)

(event `Enemy shooting`
  ;[0 0 0] Enemy aim
  (`SceneComponent.K2_SetWorldRotation` (`self.ProjectileSpawnPoint`) (`KismetMathLibrary.FindLookAtRotation` (`SceneComponent.K2_GetComponentLocation` (`self.ProjectileSpawnPoint`)) (`CharacterMovementComponent.GetLastUpdateLocation` (`Character.CharacterMovement` (`self.BubbleREF`)))) false false))

(fn `UserConstructionScript`)